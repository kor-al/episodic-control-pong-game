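; Pong game mode that runs the match: it spawns balls, tracks player and CPU scores on a HUD widget, and toggles pause.
; On start it spawns a screen capturer and, when IsVAE is set, a Python trainer actor that receives a reference to it.
; Balls launch along X at a random angle around Y, with direction random at first and then set by the last scorer.
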(event `self.ReceiveBeginPlay`
  (bind _returnvalue (`|SpawnActorFromClass` "/Game/Blueprints/ScreenCapturer_BP.ScreenCapturer_BP_C" (`KismetMathLibrary.MakeTransform` (0.0 0.0 0.0) (struct) (0.25 0.25 0.25)) "AdjustIfPossibleButDontSpawnIfColliding" "OverrideRootScale"))
  (if (`self.isVAE`)
    (bind _returnvalue_2 (`|SpawnActorFromClass` "/Game/Blueprints/PyTrainer_BP.PyTrainer_BP_C" (`KismetMathLibrary.MakeTransform` (0.0 0.0 0.0)) "Undefined" "OverrideRootScale"))
    (set `/Game/Blueprints/PyTrainer_BP.ScreenCapturer_Ref` _returnvalue _returnvalue_2))
  (set `self.ScreenCapturer` _returnvalue)
  (set `self.GameIsPaused?` true)
  (set `self.Direction` (`KismetMathLibrary.SignOfFloat` (`KismetMathLibrary.RandomFloatInRange` -1.0 1.0)))
  (`self.SpanwNewBallEvent`)
  (bind _returnvalue_3 (`|CreateWidget` "/Game/Blueprints/HUD_WG.HUD_WG_C"))
  (bind _output_get (set `self.HUD_Ref` _returnvalue_3))
  (`UserWidget.AddToViewport` _output_get 0))

(event `SpanwNewBallEvent`
  (bind _returnvalue (`|SpawnActorFromClass` "/Game/Blueprints/Ball_BP.Ball_BP_C" (`KismetMathLibrary.MakeTransform` (0.0 0.0 0.0) (struct) (0.25 0.25 0.25)) "AdjustIfPossibleButDontSpawnIfColliding" "OverrideRootScale"))
  (bind _output_get (set `self.Ball_Ref` _returnvalue))
  (bind _asball_bp (cast `/Game/Blueprints/Ball_BP` _output_get))
  (set `MovementComponent.Velocity` (`KismetMathLibrary.RotateAngleAxis` (* (1.0 0.0 0.0) (* (`self.Direction`) (`self.BallSpeed`))) (`KismetMathLibrary.RandomFloatInRange` -30.0 30.0) (0.0 1.0 0.0)) (`/Game/Blueprints/Ball_BP.ProjectileMovement` _asball_bp)))

(event `Update Player Score`
  (bind _output_get (set `self.Player_Score` (+ (`self.Player_Score`) 1)))
  (`/Game/Blueprints/HUD_WG.Update Player Score Text` (`self.HUD_Ref`) _output_get)
  (set `self.Direction` -1.0))

(event `Update Cpu Score`
  (bind _output_get (set `self.Cpu_Score` (+ (`self.Cpu_Score`) 1)))
  (`/Game/Blueprints/HUD_WG.Update Cpu Score Text` (`self.HUD_Ref`) _output_get)
  (set `self.Direction` 1.0))

(event `Pause Game Event`
  (if (`self.GameIsPaused?`)
    (set `self.GameIsPaused?` false)
    (`GameplayStatics.SetGamePaused` false)
    (`Widget.SetVisibility` (`/Game/Blueprints/HUD_WG.Paused_Text` (`self.HUD_Ref`)) "Hidden")
    (else
      (set `self.GameIsPaused?` true)
      (`Widget.SetVisibility` (`/Game/Blueprints/HUD_WG.Paused_Text` (`self.HUD_Ref`)) "Visible")
      (`GameplayStatics.SetGamePaused` true))))

(fn `UserConstructionScript`)